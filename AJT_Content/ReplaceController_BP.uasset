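; Controller actor that randomizes item placement in the level at BeginPlay, using ReplaceMe_BP actors as placeholder spots.
; It sorts placeholders by rarity into low, high and key pools, spawning fixed item sets for low and high and gathering existing Key actors for key.
; GeneralReplace shuffles each item set and its placeholders, teleports items onto them with random yaw, then destroys every placeholder, including unused ones.
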(event EventBeginPlay
  (bind _outactors (Actor|GetAllActorsOfClass "/Game/UE5_FinalProject/AJT_Content/ReplaceMe_BP.ReplaceMe_BP_C"))
  (for _array_element _outactors
    (if (Utilities|Enum|Equal(Enum) (Variables|/Game/UE5_FinalProject/AJT_Content/ReplaceMe_BP.ReplaceMe_BP_C|GetthisRarity _array_element) "NewEnumerator0")
      (Utilities|Array|Add (Variables|Default|GettoReplaceLow) _array_element)
      (elif (Utilities|Enum|Equal(Enum) (Variables|/Game/UE5_FinalProject/AJT_Content/ReplaceMe_BP.ReplaceMe_BP_C|GetthisRarity _array_element) "NewEnumerator1")
        (Utilities|Array|Add (Variables|Default|GettoReplaceHigh) _array_element)
        (else
          (Utilities|Array|Add (Variables|Default|GettoReplaceKey) _array_element)))))
  (bind _newparam (CallFunction|MakeLowRarity))
  (CallFunction|GeneralReplace _newparam (Variables|Default|GettoReplaceLow))
  (bind _newparam_2 (CallFunction|MakeHighRarity))
  (CallFunction|GeneralReplace _newparam_2 (Variables|Default|GettoReplaceHigh))
  (bind _newparam_3 (CallFunction|MakeKeyRarity))
  (CallFunction|GeneralReplace _newparam_3 (Variables|Default|GettoReplaceKey)))

(event Collision|EventActorBeginOverlap
  (params (OtherActor :type Actor%20Object%20Reference)))

(event EventTick
  (params (DeltaSeconds :type Float%20%28single-precision%29)))

(fn ConstructionScript)

(fn MakeHighRarity
  (bind _returnvalue (Game|SpawnActorfromClass "/Game/UE5_FinalProject/JOB_Content/BP_Metal_Scrap.BP_Metal_Scrap_C" (Math|Transform|MakeTransform "0, 0, 0" "0, 0, 0" "1.000000,1.000000,1.000000") "Undefined" "MultiplyWithRoot" 0 0))
  (bind _returnvalue_2 (Game|SpawnActorfromClass "/Game/UE5_FinalProject/JOB_Content/BP_Metal_Scrap.BP_Metal_Scrap_C" (Math|Transform|MakeTransform "0, 0, 0" "0, 0, 0" "1.000000,1.000000,1.000000") "Undefined" "MultiplyWithRoot" 0 0))
  (bind _returnvalue_3 (Game|SpawnActorfromClass "/Game/UE5_FinalProject/JOB_Content/BP_Metal_Scrap.BP_Metal_Scrap_C" (Math|Transform|MakeTransform "0, 0, 0" "0, 0, 0" "1.000000,1.000000,1.000000") "Undefined" "MultiplyWithRoot" 0 0))
  (bind _returnvalue_4 (Game|SpawnActorfromClass "/Game/UE5_FinalProject/JOB_Content/BP_Paper.BP_Paper_C" (Math|Transform|MakeTransform "0, 0, 0" "0, 0, 0" "1.000000,1.000000,1.000000") "Undefined" "MultiplyWithRoot" 0 0))
  (bind _returnvalue_5 (Game|SpawnActorfromClass "/Game/UE5_FinalProject/JOB_Content/BP_Paper.BP_Paper_C" (Math|Transform|MakeTransform "0, 0, 0" "0, 0, 0" "1.000000,1.000000,1.000000") "Undefined" "MultiplyWithRoot" 0 0))
  (bind _returnvalue_6 (Game|SpawnActorfromClass "/Game/UE5_FinalProject/JOB_Content/BP_Glue.BP_Glue_C" (Math|Transform|MakeTransform "0, 0, 0" "0, 0, 0" "1.000000,1.000000,1.000000") "Undefined" "MultiplyWithRoot" 0 0))
  (bind _returnvalue_7 (Game|SpawnActorfromClass "/Game/UE5_FinalProject/JOB_Content/BP_Glue.BP_Glue_C" (Math|Transform|MakeTransform "0, 0, 0" "0, 0, 0" "1.000000,1.000000,1.000000") "Undefined" "MultiplyWithRoot" 0 0))
  (return (Utilities|Array|MakeArray _returnvalue _returnvalue_2 _returnvalue_4 _returnvalue_5 _returnvalue_6 _returnvalue_7 _returnvalue_3)))

(fn GeneralReplace
  (params (PutIn :type Array%20of%20Actor%20Object%20References) (Replace :type Array%20of%20Replace%20Me%20BP%20Object%20References))
  (Utilities|Array|Shuffle PutIn)
  (Utilities|Array|Shuffle Replace)
  (for (_array_element _array_index) PutIn
    (Transformation|SetActorLocationAndRotation _array_element (Transformation|GetActorLocation (Utilities|Array|Get(acopy) Replace _array_index)) (Math|Rotator|MakeRotator 0.0 0.0 (Math|Conversions|ToFloat(Integer) (Math|Random|RandomInteger 360))) false true))
  (for _array_element_2 Replace
    (Actor|DestroyActor _array_element_2)))

(fn MakeLowRarity
  (bind _returnvalue (Game|SpawnActorfromClass "/Game/HorrorEngine/Blueprints/UsableAssets/Inventory/Flashlight.Flashlight_C" (Math|Transform|MakeTransform "0, 0, 0" "0, 0, 0" "1.000000,1.000000,1.000000") "Undefined" "MultiplyWithRoot" 0 0))
  (bind _returnvalue_2 (Game|SpawnActorfromClass "/Game/UE5_FinalProject/JOB_Content/BP_Metal_Scrap.BP_Metal_Scrap_C" (Math|Transform|MakeTransform "0, 0, 0" "0, 0, 0" "1.000000,1.000000,1.000000") "Undefined" "MultiplyWithRoot" 0 0))
  (bind _returnvalue_3 (Game|SpawnActorfromClass "/Game/UE5_FinalProject/JOB_Content/BP_Metal_Scrap.BP_Metal_Scrap_C" (Math|Transform|MakeTransform "0, 0, 0" "0, 0, 0" "1.000000,1.000000,1.000000") "Undefined" "MultiplyWithRoot" 0 0))
  (bind _returnvalue_4 (Game|SpawnActorfromClass "/Game/UE5_FinalProject/JOB_Content/BP_Metal_Scrap.BP_Metal_Scrap_C" (Math|Transform|MakeTransform "0, 0, 0" "0, 0, 0" "1.000000,1.000000,1.000000") "Undefined" "MultiplyWithRoot" 0 0))
  (bind _returnvalue_5 (Game|SpawnActorfromClass "/Game/UE5_FinalProject/JOB_Content/BP_Paper.BP_Paper_C" (Math|Transform|MakeTransform "0, 0, 0" "0, 0, 0" "1.000000,1.000000,1.000000") "Undefined" "MultiplyWithRoot" 0 0))
  (bind _returnvalue_6 (Game|SpawnActorfromClass "/Game/UE5_FinalProject/JOB_Content/BP_Paper.BP_Paper_C" (Math|Transform|MakeTransform "0, 0, 0" "0, 0, 0" "1.000000,1.000000,1.000000") "Undefined" "MultiplyWithRoot" 0 0))
  (return (Utilities|Array|MakeArray _returnvalue _returnvalue_5 _returnvalue_2 _returnvalue_3 _returnvalue_6 _returnvalue_4)))

(fn MakeKeyRarity
  (bind _outactors (Actor|GetAllActorsOfClass "/Game/HorrorEngine/Blueprints/UsableAssets/Inventory/Key.Key_C"))
  (return _outactors))